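; BP_ConfigPropertyColor is a config property that represents a linear color as four float sub-properties.
; It looks up its R, G, B and A children by key through a config section conversion and casts each to BP_ConfigPropertyFloat.
; GetColorValue assembles those values into a LinearColor, and SetColorValue writes a color's channels back into them.
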(fn GetColorValue
  (bind (_r _g _b _a) (CallFunction|GetColorProperties))
  (return (Utilities|Struct|MakeLinearColor (Variables|/Script/SML.ConfigPropertyFloat|GetValue _r) (Variables|/Script/SML.ConfigPropertyFloat|GetValue _g) (Variables|/Script/SML.ConfigPropertyFloat|GetValue _b) (Variables|/Script/SML.ConfigPropertyFloat|GetValue _a))))

(fn GetColorProperties
  (bind _self self)
  (return (.AsBP%20Config%20Property%20Float (Utilities|Casting|CastToBP_ConfigPropertyFloat (Class|RuntimeBlueprintFunctionLibrary|ToConfigProperty(ConfigPropertySection) _self "R"))) (.AsBP%20Config%20Property%20Float (Utilities|Casting|CastToBP_ConfigPropertyFloat (Class|RuntimeBlueprintFunctionLibrary|ToConfigProperty(ConfigPropertySection) _self "G"))) (.AsBP%20Config%20Property%20Float (Utilities|Casting|CastToBP_ConfigPropertyFloat (Class|RuntimeBlueprintFunctionLibrary|ToConfigProperty(ConfigPropertySection) _self "B"))) (.AsBP%20Config%20Property%20Float (Utilities|Casting|CastToBP_ConfigPropertyFloat (Class|RuntimeBlueprintFunctionLibrary|ToConfigProperty(ConfigPropertySection) _self "A")))))

(fn SetColorValue
  (params (NewValue :type Linear%20Color%20Structure))
  (bind (_r _g _b _a) (Utilities|Struct|BreakLinearColor NewValue))
  (bind (_r_2 _g_2 _b_2 _a_2) (CallFunction|GetColorProperties))
  (Variables|/Script/SML.ConfigPropertyFloat|SetValue _r_2 _r)
  (Variables|/Script/SML.ConfigPropertyFloat|SetValue _g_2 _g)
  (Variables|/Script/SML.ConfigPropertyFloat|SetValue _b_2 _b)
  (Variables|/Script/SML.ConfigPropertyFloat|SetValue _a_2 _a))