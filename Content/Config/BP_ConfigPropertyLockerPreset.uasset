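; BP_ConfigPropertyLockerPreset is a config property that stores one locker preset: a key paired with player customization data.
; It resolves itself as a config section and casts its "Key" and "Data" children to string and player customization data properties.
; The get and set functions convert between those child properties and a LockerPreset struct, delegating the customization part to the Data property's own accessors.
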(fn GetLockerPresetProperties
  (bind _self self)
  (return (.AsBP%20Config%20Property%20String (Utilities|Casting|CastToBP_ConfigPropertyString (Class|RuntimeBlueprintFunctionLibrary|ToConfigProperty(ConfigPropertySection) _self "Key"))) (.AsBP%20Config%20Property%20Player%20Customization%20Data (Utilities|Casting|CastToBP_ConfigPropertyPlayerCustomizationData (Class|RuntimeBlueprintFunctionLibrary|ToConfigProperty(ConfigPropertySection) _self "Data")))))

(fn SetLockerPresetValue
  (params (NewValue :type Locker%20Preset%20Structure))
  (bind (_key _data) (Utilities|Struct|BreakLockerPreset NewValue))
  (bind (_key_2 _data_2) (CallFunction|GetLockerPresetProperties))
  (Variables|/Script/SML.ConfigPropertyString|SetValue _key_2 _key)
  (Default|SetCustomizationValue _data_2 _data))

(fn GetLockerPresetValue
  (bind (_key _data) (CallFunction|GetLockerPresetProperties))
  (return (Utilities|Struct|MakeLockerPreset (Variables|/Script/SML.ConfigPropertyString|GetValue _key) (Default|GetCustomizationValue _data))))