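; BP_ConfigPropertyLockerPresetArrayMap is a config array property that stores locker presets as a key-addressed map.
; FindPreset linearly scans elements cast to BP_ConfigPropertyLockerPreset, matching keys and returning the preset, property and index, or -1.
; AddPreset overwrites a matching preset or appends a new element, while GetPreset, RemovePreset and GetAllPresets handle lookup, deletion and full listing.
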(fn FindPreset
  (params (Key :type String))
  (for (_array_element _array_index) (Class|RuntimeBlueprintFunctionLibrary|ToConfigPropertyArray(ConfigPropertyArray) self)
    (bind _asbp_config_property_locker_preset (Utilities|Casting|CastToBP_ConfigPropertyLockerPreset _array_element))
    (if (CallFunction|PresetKeyEqual (Default|GetLockerPresetValue _asbp_config_property_locker_preset) Key)
      (return (Default|GetLockerPresetValue _asbp_config_property_locker_preset) _asbp_config_property_locker_preset _array_index)))
  (return "" 0 -1))

(fn PresetKeyEqual
  (params (Preset :type Locker%20Preset%20Structure) (Key :type String))
  (return (Utilities|Enum|Equal(Enum) (.Key (Utilities|Struct|BreakLockerPreset Preset)) Key)))

(fn RemovePreset
  (params (Key :type String))
  (bind _index (CallFunction|FindPreset Key))
  (Class|ConfigPropertyArray|RemoveElementatIndex _index))

(fn GetAllPresets
  (for _array_element (Class|RuntimeBlueprintFunctionLibrary|ToConfigPropertyArray(ConfigPropertyArray) self)
    (Utilities|Array|Add (LocalVariables|GetLocalPresets) (Default|GetLockerPresetValue (.AsBP%20Config%20Property%20Locker%20Preset (Utilities|Casting|CastToBP_ConfigPropertyLockerPreset _array_element)))))
  (return (LocalVariables|GetLocalPresets)))

(fn AddPreset
  (params (Preset :type Locker%20Preset%20Structure))
  (bind (_preset _property _index) (CallFunction|FindPreset (.Key (Utilities|Struct|BreakLockerPreset Preset))))
  (if (>= _index 0)
    _
    (else
      (bind _returnvalue (Class|ConfigPropertyArray|AddNewElement))
      (bind _asbp_config_property_locker_preset (Utilities|Casting|CastToBP_ConfigPropertyLockerPreset _returnvalue))))
  (Default|SetLockerPresetValue _asbp_config_property_locker_preset Preset))

(fn GetPreset
  (params (Key :type String))
  (bind (_preset _property _index) (CallFunction|FindPreset Key))
  (return _preset (>= _index 0)))