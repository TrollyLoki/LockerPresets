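; Config property section that stores player customization data: three colors, helmet and trinket descriptors, and equipment skins.
; GetCustomizationProperties looks up child properties by key and casts them to typed color, class and array properties.
; GetCustomizationValue packs these into a PlayerCustomizationData struct, casting classes to their descriptor types.
; SetCustomizationValue writes a struct back into the properties, clearing and rebuilding the equipment array element by element.
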(fn GetCustomizationProperties
  (bind _self self)
  (return (.AsBP%20Config%20Property%20Color (Utilities|Casting|CastToBP_ConfigPropertyColor (Class|RuntimeBlueprintFunctionLibrary|ToConfigProperty(ConfigPropertySection) _self "PrimaryColor"))) (.AsBP%20Config%20Property%20Color (Utilities|Casting|CastToBP_ConfigPropertyColor (Class|RuntimeBlueprintFunctionLibrary|ToConfigProperty(ConfigPropertySection) _self "SecondaryColor"))) (.AsBP%20Config%20Property%20Color (Utilities|Casting|CastToBP_ConfigPropertyColor (Class|RuntimeBlueprintFunctionLibrary|ToConfigProperty(ConfigPropertySection) _self "DetailColor"))) (.AsBP%20Config%20Property%20Class (Utilities|Casting|CastToBP_ConfigPropertyClass (Class|RuntimeBlueprintFunctionLibrary|ToConfigProperty(ConfigPropertySection) _self "HelmetCustomizationDesc"))) (.AsBP%20Config%20Property%20Class (Utilities|Casting|CastToBP_ConfigPropertyClass (Class|RuntimeBlueprintFunctionLibrary|ToConfigProperty(ConfigPropertySection) _self "TrinketCustomizationDesc"))) (.AsBP%20Config%20Property%20Array (Utilities|Casting|CastToBP_ConfigPropertyArray (Class|RuntimeBlueprintFunctionLibrary|ToConfigProperty(ConfigPropertySection) _self "EquipmentCustomizationDesc")))))

(fn GetCustomizationValue
  (bind (_primarycolor _secondarycolor _detailcolor _helmetcustomizationdesc _trinketcustomizationdesc _equipmentcustomizationdesc) (CallFunction|GetCustomizationProperties))
  (bind _equipmentskins (LocalVariables|GetEquipmentSkins))
  (for _array_element (Variables|/Script/SML.ConfigPropertyArray|GetValues _equipmentcustomizationdesc)
    (Utilities|Array|Add _equipmentskins (.AsFGPlayer%20Equipment%20Skin%20Customization%20Desc (Utilities|Casting|CastToFGPlayerEquipmentSkinCustomizationDescClass (Variables|/Script/SML.ConfigPropertyClass|GetValue (.AsBP%20Config%20Property%20Class (Utilities|Casting|CastToBP_ConfigPropertyClass _array_element)))))))
  (return (Utilities|Struct|MakePlayerCustomizationData (Default|GetColorValue _primarycolor) (Default|GetColorValue _secondarycolor) (Default|GetColorValue _detailcolor) (.AsFGPlayer%20Helmet%20Customization%20Desc (Utilities|Casting|CastToFGPlayerHelmetCustomizationDescClass (Variables|/Script/SML.ConfigPropertyClass|GetValue _helmetcustomizationdesc))) (.AsFGPlayer%20Trinket%20Customization%20Desc (Utilities|Casting|CastToFGPlayerTrinketCustomizationDescClass (Variables|/Script/SML.ConfigPropertyClass|GetValue _trinketcustomizationdesc))) _equipmentskins)))

(fn SetCustomizationValue
  (params (NewValue :type Player%20Customization%20Data%20Structure))
  (bind (_primarycolor _secondarycolor _detailcolor _helmetcustomizationdesc _trinketcustomizationdesc _equipmentcustomizationdesc) (Utilities|Struct|BreakPlayerCustomizationData NewValue))
  (bind (_primarycolor_2 _secondarycolor_2 _detailcolor_2 _helmetcustomizationdesc_2 _trinketcustomizationdesc_2 _equipmentcustomizationdesc_2) (CallFunction|GetCustomizationProperties))
  (Default|SetColorValue _primarycolor_2 _primarycolor)
  (Default|SetColorValue _secondarycolor_2 _secondarycolor)
  (Default|SetColorValue _detailcolor_2 _detailcolor)
  (Class|ConfigPropertyClass|SetClassValue _helmetcustomizationdesc_2 _helmetcustomizationdesc)
  (Class|ConfigPropertyClass|SetClassValue _trinketcustomizationdesc_2 _trinketcustomizationdesc)
  (Class|ConfigPropertyArray|Clear _equipmentcustomizationdesc_2)
  (for _array_element _equipmentcustomizationdesc
    (bind _returnvalue (Class|ConfigPropertyArray|AddNewElement _equipmentcustomizationdesc_2))
    (Class|ConfigPropertyClass|SetClassValue (.AsBP%20Config%20Property%20Class (Utilities|Casting|CastToBP_ConfigPropertyClass _returnvalue)) _array_element)))